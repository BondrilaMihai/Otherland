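; Player character Blueprint for a 2D side-scrolling Paper2D game, shown with a HUD only on the level named Map.
; Axis input moves along X, turning the controller and flipbook sprite, while a simple state gates jumping.
; Capsule hits trigger damage with camera shake, a brief freeze of input and the hit actor's tick, then knockback.
; Escape opens a pause widget; other keys apply self-damage or teleport, apparently as debug shortcuts.
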(event `self.ReceiveBeginPlay`
  ;[1 1 1] Begin Play
  (bind _returnvalue (`GameplayStatics.GetCurrentLevelName` true))
  (if (`KismetStringLibrary.EqualEqual_StrStr` _returnvalue "Map")
    (`self.SetActorHiddenInGame` false)
    (bind _returnvalue_2 (`|CreateWidget` "/Game/Game/Blueprints/HUD/HUD.HUD_C" (`GameplayStatics.GetPlayerController` 0)))
    (`UserWidget.AddToViewport` _returnvalue_2 0)
    (else
      (`self.SetActorHiddenInGame` true))))

(event `Key|Escape`
  (params (Key :type "Key Structure"))
  (bind _returnvalue (`GameplayStatics.GetPlayerController` 0))
  ;[1 1 1] Pause Game
  (:`Pressed`
    (`GameplayStatics.SetGamePaused` true)
    (bind _returnvalue_2 (`|CreateWidget` "/Game/Game/Blueprints/GUI/InGamePause.InGamePause_C" _returnvalue))
    (`UserWidget.AddToViewport` _returnvalue_2 0)
    (set `PlayerController.bShowMouseCursor` true _returnvalue)
    (`WidgetBlueprintLibrary.SetInputMode_UIOnlyEx` _returnvalue _returnvalue_2)))

(event `Key|I`
  (params (Key :type "Key Structure"))
  (:`Pressed`
    (`self.TakeDamage` 100)))

(event `RotateController`
  (bind _returnvalue (`self.GetController`))
  ;[1 1 1] Rotate Controller
  (`/Engine/EditorBlueprintResources/StandardMacros.CompareFloat` (.x (`MovementComponent.Velocity` (`self.GetMovementComponent`)))
    (:`>`
      (`Controller.SetControlRotation` _returnvalue (`KismetMathLibrary.MakeRotator` 0.0 0.0 180.0) :!label _label))
    (:`==`
      (if (`self.BisMovingRight`)
        (goto _label)
        (else
          (`Controller.SetControlRotation` _returnvalue (`KismetMathLibrary.MakeRotator` 0.0) :!label _label_2))))
    (:`<`
      (goto _label_2))))

(event `Update Sprite`
  (bind _sprite (`self.Sprite`))
  ;[1 1 1] Update Sprite
  (`SceneComponent.K2_SetRelativeRotation` _sprite (`self.GetControlRotation`) false false)
  (`PaperFlipbookComponent.SetFlipbook` _sprite (select `bool` (> (`KismetMathLibrary.VSize` (`self.GetVelocity`)) 0.0) :`false` "/Game/Game/Sprites/PlayerFlipbooks/A_Idle.A_Idle" :`true` "/Game/Game/Sprites/PlayerFlipbooks/A_Idle.A_Idle" :!type "PaperFlipbook Object Reference")))

(event `TakeDamage`
  (params (DamageAmount :type Integer) (HitActor :type "Actor Object Reference"))
  (bind _returnvalue (`GameplayStatics.GetPlayerController` 0))
  ;[1 1 1] TakeDamage
  (`self.DisableInput` _returnvalue)
  (`self.SetActorTickEnabled` HitActor false)
  (`PlayerCameraManager.PlayCameraShake` :`self` (`GameplayStatics.GetPlayerCameraManager` 0) :`ShakeClass` "/Game/Game/Blueprints/Player/PlayerDamageShake.PlayerDamageShake_C")
  (`KismetSystemLibrary.Delay` 0.5)
  (`self.EnableInput` _returnvalue)
  (`self.SetActorTickEnabled` HitActor true)
  (`self.MyTakeDamage` DamageAmount)
  (if (`self.BisMovingRight`)
    (set `self.BisMovingRight` false)
    (`self.LaunchCharacter` (-500.0 0.0 300.0) true true)
    (else
      (set `self.BisMovingRight` true)
      (`self.LaunchCharacter` (500.0 0.0 300.0) true true))))

(event `Key|F`
  (params (Key :type "Key Structure"))
  (:`Pressed`
    (bind _outactors (`GameplayStatics.GetAllActorsOfClass` "/Script/Engine.PlayerStart"))
    (for _array_element _outactors
      (if (== (`PlayerStart.PlayerStartTag` _array_element) "Assassins")
        (`self.K2_TeleportTo` (`self.K2_GetActorLocation` _array_element))))))

(event `self.CapsuleComponent.OnComponentHit`
  (params (HitComponent :type "PrimitiveComponent Object Reference") (OtherActor :type "Actor Object Reference") (OtherComp :type "PrimitiveComponent Object Reference") (NormalImpulse :type "Vector Structure") (Hit :type "HitResult Structure (by ref)"))
  (if (== (`GameplayStatics.GetObjectClass` OtherActor) null)
    (`self.TakeDamage` 100 OtherActor)))

(event `InputAxis|MoveRight`
  (params (AxisValue :type "Float (single-precision)"))
  ;[1 1 1] Moving Sideways
  (if (> AxisValue 0.0)
    (set `self.BisMovingRight` true)
    (elif (< AxisValue 0.0)
      (set `self.BisMovingRight` false)))
  (`self.RotateController`)
  (`self.Update Sprite`)
  (`self.AddMovementInput` (1.0 0.0 0.0) AxisValue))

(event `Key|Z`
  (params (Key :type "Key Structure"))
  (:`Pressed`
    (`self.K2_TeleportTo` (-17899.0 0.0 4500.0))))

(event `InputAction|Jump`
  (params (Key :type "Key Structure"))
  ;[1 1 1] Handle Jump
  (:`Pressed`
    (if (`|EnumEquality` (`self._characterState`) "State_Idle")
      (set `self._characterState` "State_Jumping")
      (`self.Jump`)))
  (:`Released`
    (`self.StopJumping`)))

(event `self.OnLanded`
  (params (Hit :type "HitResult Structure (by ref)"))
  ;[1 1 1] Handle Jump
  (set `self._characterState` "State_Idle"))

(fn `UserConstructionScript`)
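; Player Blueprint for a 2D side-scrolling flipbook character that moves along the X axis and jumps.
; MoveRight input turns the controller by X velocity, or last input direction when stopped, then matches sprite rotation to it; the flipbook is always A_Idle.
; A PlayerState enum blocks jumping again until OnLanded resets it to idle.
; The F key teleports to the "Assassins"-tagged PlayerStart, and Z to a fixed location.
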(event `RotateController`
  (bind _returnvalue (`self.GetController`))
  ;[1 1 1] Rotate Controller
  (`/Engine/EditorBlueprintResources/StandardMacros.CompareFloat` (.x (`MovementComponent.Velocity` (`self.GetMovementComponent`)))
    (:`>`
      (`Controller.SetControlRotation` _returnvalue (`KismetMathLibrary.MakeRotator` 0.0 0.0 180.0) :!label _label))
    (:`==`
      (if (`self.BisMovingRight`)
        (goto _label)
        (else
          (`Controller.SetControlRotation` _returnvalue (`KismetMathLibrary.MakeRotator` 0.0) :!label _label_2))))
    (:`<`
      (goto _label_2))))

(event `Update Sprite`
  (bind _sprite (`self.Sprite`))
  ;[1 1 1] Update Sprite
  (`SceneComponent.K2_SetRelativeRotation` _sprite (`self.GetControlRotation`) false false)
  (`PaperFlipbookComponent.SetFlipbook` _sprite (select `bool` (> (`KismetMathLibrary.VSize` (`self.GetVelocity`)) 0.0) :`false` "/Game/Game/Sprites/PlayerFlipbooks/A_Idle.A_Idle" :`true` "/Game/Game/Sprites/PlayerFlipbooks/A_Idle.A_Idle" :!type "PaperFlipbook Object Reference")))

(event `Key|F`
  (params (Key :type "Key Structure"))
  (:`Pressed`
    (bind _outactors (`GameplayStatics.GetAllActorsOfClass` "/Script/Engine.PlayerStart"))
    (for _array_element _outactors
      (if (== (`PlayerStart.PlayerStartTag` _array_element) "Assassins")
        (`self.K2_TeleportTo` (`self.K2_GetActorLocation` _array_element))))))

(event `InputAxis|MoveRight`
  (params (AxisValue :type "Float (single-precision)"))
  ;[1 1 1] Moving Sideways
  (if (> AxisValue 0.0)
    (set `self.BisMovingRight` true)
    (elif (< AxisValue 0.0)
      (set `self.BisMovingRight` false)))
  (`self.RotateController`)
  (`self.Update Sprite`)
  (`self.AddMovementInput` (1.0 0.0 0.0) AxisValue))

(event `Key|Z`
  (params (Key :type "Key Structure"))
  (:`Pressed`
    (`self.K2_TeleportTo` (-17899.0 0.0 4500.0))))

(event `self.ReceiveTick`
  (params (DeltaSeconds :type "Float (single-precision)")))

(event `InputAction|Jump`
  (params (Key :type "Key Structure"))
  ;[1 1 1] Handle Jump
  (:`Pressed`
    (if (`|EnumEquality` (`self._playerState`) "State_Idle")
      (set `self._playerState` "State_Jumping")
      (`self.Jump`)))
  (:`Released`
    (`self.StopJumping`)))

(event `self.OnLanded`
  (params (Hit :type "HitResult Structure (by ref)"))
  ;[1 1 1] Handle Jump
  (set `self._playerState` "State_Idle"))

(fn `UserConstructionScript`)
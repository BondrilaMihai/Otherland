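; Flipbook-sprite assassin boss, apparently work in progress, driven by random decisions on Tick and a state enum.
; Tick prints the state, then occasionally calls Decide, which can trigger DaggerTp from the default state, or otherwise refreshes the idle animation.
; DaggerTp plays its flipbook for that clip's length, then restores idle, without moving the actor.
; Shadowstep collision swapping, jump, landing reset and facing rotation exist only as unconnected logic.
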(event `self.K2_OnMovementModeChanged`
  (params (PrevMovementMode :type "EMovementMode Enum" :default "MOVE_None") (NewMovementMode :type "EMovementMode Enum" :default "MOVE_None") (PrevCustomMode :type Byte) (NewCustomMode :type Byte)))

(event `UpdateAnimation`
  ;[1 1 1] Handle Animation
  (`PaperFlipbookComponent.SetFlipbook` (`self.Sprite`) (select `bool` (> (`KismetMathLibrary.VSize` (`self.GetVelocity`)) 0.0) :`false` "/Game/Game/Sprites/AssassinsSprites/Boss/A_Idle.A_Idle" :`true` "/Game/Game/Sprites/AssassinsSprites/Boss/A_Idle.A_Idle" :!type "PaperFlipbook Object Reference")))

(event `Decide`
  (bind _returnvalue (`KismetMathLibrary.RandomIntegerInRange` 0 100))
  (`self.SetActorTickEnabled` false)
  (if (<= _returnvalue 40)
    _
    (elif (and (> _returnvalue 40) (<= _returnvalue 70))
      (if (`|EnumEquality` (`self.State`) "NewEnumerator0")
        (`self.DaggerTp`))))
  (`self.SetActorTickEnabled` true))

(event `self.ReceiveBeginPlay`
  ;[1 1 1] Begin Play
  (set `self.State` "NewEnumerator0"))

(event `DaggerTp`
  (bind _sprite (`self.Sprite`))
  (set `self.State` "NewEnumerator4")
  (`PaperFlipbookComponent.SetFlipbook` _sprite "/Game/Game/Sprites/AssassinsSprites/Boss/DaggerTp/A_DaggerTp.A_DaggerTp")
  (`KismetSystemLibrary.Delay` (`PaperFlipbookComponent.GetFlipbookLength` _sprite))
  (`PaperFlipbookComponent.SetFlipbook` _sprite "/Game/Game/Sprites/AssassinsSprites/Boss/A_Idle.A_Idle")
  (set `self.State` "NewEnumerator0"))

(event `InputAxis|MoveRight`
  (params (AxisValue :type "Float (single-precision)"))
  ;[1 1 1] Handle Movement
  (if (> AxisValue 0.0)
    (set `self.bisMovingRight` true)
    (elif (< AxisValue 0.0)
      (set `self.bisMovingRight` false)))
  (`self.AddMovementInput` (0.0 0.0 0.0) AxisValue))

(event `self.ReceiveTick`
  (params (DeltaSeconds :type "Float (single-precision)"))
  ;[1 1 1] Tick - Updates Animation
  (`KismetSystemLibrary.PrintString` (`|GetEnumeratorNameAsString` (`self.State`)))
  (if (<= (`KismetMathLibrary.RandomIntegerInRange` 0 100) 2)
    (`self.Decide`)
    (else
      (`self.UpdateAnimation`))))

(fn `UserConstructionScript`)
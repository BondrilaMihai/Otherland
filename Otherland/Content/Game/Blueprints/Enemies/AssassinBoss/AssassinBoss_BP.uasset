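; Assassin boss enemy that faces the player, takes damage from their attacks and hands back the music when defeated.
; Tick keeps AI focus on the player, prints its state and sets the idle flipbook.
; Capsule overlaps deal damage scaled by the player's spirit-drop or attack state, with hurt sprite and sound.
; Death disables player input, stops ambient sounds, then after a delay switches them to the Assassins cue, restores input and destroys the boss.
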(event `Die`
  ;[1 1 1] Die
  (`self.DisableInput` (`GameplayStatics.GetPlayerCharacter` 0) null)
  (`self.SetActorTickEnabled` false)
  (`PaperFlipbookComponent.SetFlipbook` (`self._sprite`) "/Game/Game/Sprites/AssassinsSprites/Boss/A_Defeated.A_Defeated")
  (bind _outactors (`GameplayStatics.GetAllActorsOfClass` "/Script/Engine.AmbientSound"))
  (for _array_element _outactors
    (`AudioComponent.Stop` (`AmbientSound.AudioComponent` _array_element))
    (`KismetSystemLibrary.Delay` 3.0)
    (bind _outactors_2 (`GameplayStatics.GetAllActorsOfClass` "/Script/Engine.AmbientSound"))
    (for _array_element_2 _outactors_2
      (bind _audiocomponent (`AmbientSound.AudioComponent` _array_element_2))
      (`AudioComponent.SetSound` _audiocomponent "/Game/Game/Audio/Soundtracks/Assassins_Cue.Assassins_Cue")
      (`AudioComponent.Play` _audiocomponent 0.0))
    (`self.EnableInput` (`GameplayStatics.GetPlayerCharacter` 0) null)
    (`self.K2_DestroyActor`)))

(event `TakeDamage`
  (params (DamageAmount :type Integer) (HitActor :type "Actor Object Reference"))
  ;[1 1 1] TakeDamage
  (`PaperFlipbookComponent.SetFlipbook` (`self._sprite`) "/Game/Game/Sprites/AssassinsSprites/Boss/A_Damaged.A_Damaged")
  (`self.MyTakeDamage` DamageAmount)
  (`GameplayStatics.SpawnSound2D` "/Game/Game/Audio/Misc/Enemy_Take_Damage_Cue.Enemy_Take_Damage_Cue" 1.0 1.0 0.0 null)
  (`KismetSystemLibrary.Delay` 0.2)
  (if (`self._isDead`)
    (`self.Die`)))

(event `FocusOnPlayer`
  ;[1 1 1] Focus on Player
  (bind _asaicontroller (cast `AIController` (`self.GetController`)))
  (`AIController.K2_SetFocus` _asaicontroller (`GameplayStatics.GetPlayerCharacter` 0)))

(event `UpdateAnimation`
  ;[1 1 1] Handle Animation
  (`PaperFlipbookComponent.SetFlipbook` (`self._sprite`) (select `bool` (> (`KismetMathLibrary.VSize` (`self.GetVelocity`)) 0.0) :`false` "/Game/Game/Sprites/AssassinsSprites/Boss/A_Idle.A_Idle" :`true` "/Game/Game/Sprites/AssassinsSprites/Boss/A_Idle.A_Idle" :!type "PaperFlipbook Object Reference")))

(event `self.ReceiveBeginPlay`)

(event `self.ReceiveTick`
  (params (DeltaSeconds :type "Float (single-precision)"))
  ;[1 1 1] Event Tick
  (`KismetSystemLibrary.PrintString` (`|GetEnumeratorNameAsString` (`self._characterState`)))
  (`self.FocusOnPlayer`)
  (`self.UpdateAnimation`))

(event `self.CapsuleComponent.OnComponentBeginOverlap`
  (params (OverlappedComponent :type "PrimitiveComponent Object Reference") (OtherActor :type "Actor Object Reference") (OtherComp :type "PrimitiveComponent Object Reference") (OtherBodyIndex :type Integer) (bFromSweep :type Boolean) (SweepResult :type "HitResult Structure (by ref)"))
  ;[1 1 1] Collision
  (if (== OtherActor (`GameplayStatics.GetPlayerCharacter` 0))
    (bind _asmy_player_bp (cast `/Game/Game/Blueprints/Player/MyPlayer_BP` OtherActor))
    (bind __characterstate (`MyCharacter._characterState` _asmy_player_bp))
    (if (`|EnumEquality` __characterstate "State_SpiritDrop")
      (`self.TakeDamage` 125)
      (elif (`|EnumEquality` __characterstate "State_DealingDamage")
        (`self.TakeDamage` 50)))))

(fn `UserConstructionScript`)
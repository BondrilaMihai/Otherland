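; Player character Blueprint for a 2D side-scroller, handling movement, jump, melee, damage, pause and map-only HUD setup.
; A CharacterState variable gates input and selects flipbooks, while controller yaw flips the sprite by direction.
; Hit events with upward normals serve as custom landing detection; boss contact triggers camera shake, a brief freeze, then knockback or death to menu.
; Hardwired keys also trigger self-damage and teleports; Shadowstep and SpiritDrop states are only read here.
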(event `Update Sprite`
  (bind _sprite (`self.Sprite`))
  (bind _sprite_2 (`self.Sprite`))
  (bind __characterstate (`self._characterState`))
  ;[1 1 1] Update Sprite
  (`SceneComponent.K2_SetRelativeRotation` _sprite (`self.GetControlRotation`) false false)
  (if (`|EnumEquality` __characterstate "State_Jumping")
    (`PaperFlipbookComponent.SetFlipbook` _sprite "/Game/Game/Sprites/PlayerFlipbooks/A_Jumping.A_Jumping")
    (elif (`|EnumEquality` __characterstate "State_Walking")
      (`PaperFlipbookComponent.SetFlipbook` _sprite "/Game/Game/Sprites/PlayerFlipbooks/Walking/A_Walking.A_Walking")
      (elif (`|EnumEquality` __characterstate "State_Idle")
        (`PaperFlipbookComponent.SetFlipbook` _sprite "/Game/Game/Sprites/PlayerFlipbooks/A_Idle.A_Idle")
        (elif (`|EnumEquality` __characterstate "State_SpiritDrop")
          (`PaperFlipbookComponent.SetFlipbook` _sprite_2 "/Game/Game/Sprites/PlayerFlipbooks/SpiritDrop/A_SpiritDrop.A_SpiritDrop")
          (elif (`|EnumEquality` __characterstate "State_DealingDamage")
            (`PaperFlipbookComponent.SetFlipbook` _sprite_2 "/Game/Game/Sprites/PlayerFlipbooks/Melee/A_Melee.A_Melee")
            (else
              (`PaperFlipbookComponent.SetFlipbook` _sprite_2 "/Game/Game/Sprites/PlayerFlipbooks/Shadowstep/A_Shadowstep.A_Shadowstep"))))))))

(event `InputAxis|MoveRight`
  (params (AxisValue :type "Float (single-precision)"))
  (bind __characterstate (`self._characterState`))
  (bind __characterstate_2 (`self._characterState`))
  (bind _iswalkingsound (`self.IsWalkingSound`))
  ;[1 1 1] Moving Sideways
  (if (`|EnumEquality` __characterstate "State_Jumping")
    _
    (elif (`|EnumEquality` __characterstate "State_Shadowstep")
      _
      (elif (`|EnumEquality` __characterstate "State_SpiritDrop")
        _
        (elif (not (`|EnumEquality` __characterstate "State_DealingDamage"))
          (set `self._characterState` "State_Walking")
          (if (not (`AudioComponent.IsPlaying` _iswalkingsound))
            (`AudioComponent.Play` _iswalkingsound 0.0))))))
  (if (> AxisValue 0.0)
    (set `self.BisMovingRight` true)
    (elif (< AxisValue 0.0)
      (set `self.BisMovingRight` false)
      (elif (`|EnumEquality` __characterstate_2 "State_Jumping")
        _
        (elif (`|EnumEquality` __characterstate_2 "State_Shadowstep")
          _
          (elif (`|EnumEquality` __characterstate_2 "State_SpiritDrop")
            _
            (elif (not (`|EnumEquality` __characterstate_2 "State_DealingDamage"))
              (`AudioComponent.Stop` _iswalkingsound)
              (set `self._characterState` "State_Idle")))))))
  (`self.RotateController`)
  (`self.Update Sprite`)
  (`self.AddMovementInput` (1.0 0.0 0.0) AxisValue))

(event `self.ReceiveBeginPlay`
  ;[1 1 1] Begin Play
  (bind _returnvalue (`GameplayStatics.GetCurrentLevelName` true))
  (if (`KismetStringLibrary.EqualEqual_StrStr` _returnvalue "Map")
    (`self.SetActorHiddenInGame` false)
    (bind _returnvalue_2 (`|CreateWidget` "/Game/Game/Blueprints/HUD/HUD.HUD_C" (`GameplayStatics.GetPlayerController` 0)))
    (`UserWidget.AddToViewport` _returnvalue_2 0)
    (bind _returnvalue_3 (`AddComponent|NODE_AddAudioComponent-0`))
    (bind _output_get (set `self.IsWalkingSound` _returnvalue_3))
    (`AudioComponent.SetSound` _output_get "/Game/Game/Audio/Player/Player_Walk_Cue.Player_Walk_Cue")
    (else
      (`self.SetActorHiddenInGame` true))))

(event `Key|Escape`
  (params (Key :type "Key Structure"))
  (bind _returnvalue (`GameplayStatics.GetPlayerController` 0))
  ;[1 1 1] Pause Game
  (:`Pressed`
    (`GameplayStatics.SetGamePaused` true)
    (bind _returnvalue_2 (`|CreateWidget` "/Game/Game/Blueprints/GUI/InGamePause.InGamePause_C" _returnvalue))
    (`UserWidget.AddToViewport` _returnvalue_2 0)
    (set `PlayerController.bShowMouseCursor` true _returnvalue)
    (`WidgetBlueprintLibrary.SetInputMode_UIOnlyEx` _returnvalue _returnvalue_2)))

(event `Key|I`
  (params (Key :type "Key Structure"))
  (:`Pressed`
    (`self.TakeDamage` 100)
    (`GameplayStatics.SpawnSound2D` "/Game/Game/Audio/Player/Player_Take_Damage_Cue.Player_Take_Damage_Cue" 1.0 1.0 0.0 null)))

(event `RotateController`
  (bind _returnvalue (`self.GetController`))
  ;[1 1 1] Rotate Controller
  (`/Engine/EditorBlueprintResources/StandardMacros.CompareFloat` (.x (`MovementComponent.Velocity` (`self.GetMovementComponent`)))
    (:`>`
      (`Controller.SetControlRotation` _returnvalue (`KismetMathLibrary.MakeRotator` 0.0 0.0 180.0) :!label _label))
    (:`==`
      (if (`self.BisMovingRight`)
        (goto _label)
        (else
          (`Controller.SetControlRotation` _returnvalue (`KismetMathLibrary.MakeRotator` 0.0) :!label _label_2))))
    (:`<`
      (goto _label_2))))

(event `Key|F`
  (params (Key :type "Key Structure"))
  (:`Pressed`
    (bind _outactors (`GameplayStatics.GetAllActorsOfClass` "/Script/Engine.PlayerStart"))
    (for _array_element _outactors
      (if (== (`PlayerStart.PlayerStartTag` _array_element) "Assassins")
        (`self.K2_TeleportTo` (`self.K2_GetActorLocation` _array_element))))))

(event `InputAction|Jump`
  (params (Key :type "Key Structure"))
  (bind __characterstate (`self._characterState`))
  ;[1 1 1] Handle Jump
  (:`Pressed`
    (if (or (`|EnumEquality` __characterstate "State_Idle") (`|EnumEquality` __characterstate "State_Walking"))
      (set `self._characterState` "State_Jumping")
      (`AudioComponent.Stop` (`self.IsWalkingSound`))
      (`GameplayStatics.SpawnSound2D` "/Game/Game/Audio/Player/Player_Jump_Cue.Player_Jump_Cue" 1.0 1.0 0.0 null)
      (`self.Jump`)
      (`self.Update Sprite`)))
  (:`Released`
    (`self.StopJumping`)))

(event `self.CapsuleComponent.OnComponentHit`
  (params (HitComponent :type "PrimitiveComponent Object Reference") (OtherActor :type "Actor Object Reference") (OtherComp :type "PrimitiveComponent Object Reference") (NormalImpulse :type "Vector Structure") (Hit :type "HitResult Structure (by ref)"))
  (if (== (`GameplayStatics.GetObjectClass` OtherActor) "/Game/Game/Blueprints/Enemies/AssassinBoss/AssassinBoss_BP.AssassinBoss_BP_C")
    (`self.TakeDamage` 100 OtherActor)
    (`GameplayStatics.SpawnSound2D` "/Game/Game/Audio/Player/Player_Take_Damage_Cue.Player_Take_Damage_Cue" 1.0 1.0 0.0 null)))

(event `Key|Z`
  (params (Key :type "Key Structure"))
  (:`Pressed`
    (`self.K2_TeleportTo` (-17899.0 0.0 4500.0))))

(event `self.ReceiveHit`
  (params (MyComp :type "PrimitiveComponent Object Reference") (Other :type "Actor Object Reference") (OtherComp :type "PrimitiveComponent Object Reference") (bSelfMoved :type Boolean) (HitLocation :type "Vector Structure") (HitNormal :type "Vector Structure") (NormalImpulse :type "Vector Structure") (Hit :type "HitResult Structure (by ref)"))
  (bind __characterstate (`self._characterState`))
  ;[1 1 1] Custom On-Landed Event
  (if (== HitNormal (0.0 0.0 1.0))
    (if (`|EnumEquality` __characterstate "State_Shadowstep")
      (`self.DisableInput` null :!label _label_3)
      (`KismetSystemLibrary.Delay` 0.3)
      (elif (`|EnumEquality` __characterstate "State_SpiritDrop")
        (`GameplayStatics.SpawnSound2D` "/Game/Game/Audio/Spells/Spirit_Drop_Impact_Cue.Spirit_Drop_Impact_Cue" 1.0 1.0 0.0 null)
        (`self.DisableInput` null)
        (`KismetSystemLibrary.Delay` 0.2)
        (else
          (`GameplayStatics.SpawnSound2D` "/Game/Game/Audio/Player/Player_land_Cue.Player_land_Cue" 1.0 1.0 0.0 null)
          (if (`|EnumEquality` __characterstate "State_Shadowstep")
            (goto _label_3)
            (else
              (`PaperFlipbookComponent.SetFlipbook` (`self.Sprite`) "/Game/Game/Sprites/PlayerFlipbooks/A_Landed.A_Landed")
              (goto _label_3))))))
    (`self.EnableInput` null)
    (if (not (`|EnumEquality` (`self._characterState`) "State_Shadowstep"))
      (set `self._characterState` "State_Idle"))))

(event `TakeDamage`
  (params (DamageAmount :type Integer) (HitActor :type "Actor Object Reference"))
  (bind _returnvalue (`GameplayStatics.GetPlayerController` 0))
  ;[1 1 1] TakeDamage
  (`PaperFlipbookComponent.SetFlipbook` (`self.Sprite`) "/Game/Game/Sprites/PlayerFlipbooks/A_Damaged.A_Damaged")
  (`self.DisableInput` _returnvalue)
  (`self.SetActorTickEnabled` HitActor false)
  (`PlayerCameraManager.PlayCameraShake` :`self` (`GameplayStatics.GetPlayerCameraManager` 0) :`ShakeClass` "/Game/Game/Blueprints/Player/PlayerDamageShake.PlayerDamageShake_C")
  (`KismetSystemLibrary.Delay` 0.5)
  (`self.EnableInput` _returnvalue)
  (`self.SetActorTickEnabled` HitActor true)
  (`self.MyTakeDamage` DamageAmount)
  (if (`self._isDead`)
    (`self.Die`)
    (elif (`self.BisMovingRight`)
      (set `self.BisMovingRight` false)
      (`self.LaunchCharacter` (-500.0 0.0 300.0) true true)
      (else
        (set `self.BisMovingRight` true)
        (`self.LaunchCharacter` (500.0 0.0 300.0) true true)))))

(event `Die`
  ;[1 1 1] On death
  (`self.DisableInput` null)
  (`KismetSystemLibrary.Delay` 2.0)
  (`GameplayStatics.OpenLevel` "MainMenui"))

(event `Key|C`
  (params (Key :type "Key Structure"))
  (bind __characterstate (`self._characterState`))
  ;[1 1 1] Melee
  (:`Pressed`
    (if (or (`|EnumEquality` __characterstate "State_Idle") (`|EnumEquality` __characterstate "State_Walking"))
      (set `self._characterState` "State_DealingDamage")
      (`GameplayStatics.PlaySound2D` "/Game/Game/Audio/Player/Player_Melee_Cue.Player_Melee_Cue" 1.0 1.0 0.0 null null)
      (`KismetSystemLibrary.Delay` 0.4)
      (set `self._characterState` "State_Idle"))))

(fn `UserConstructionScript`)
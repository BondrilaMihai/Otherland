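; Side-scrolling 2D player character with axis movement, jumping, a downward Spirit Slam and a timed Shadowstep.
; Tick updates the flipbook (idle in both cases) and turns the controller to face movement; Shadowstep temporarily swaps collision channel and blocks jumping.
; BeginPlay teleports to the HUB PlayerStart, with F and Z as teleport keys.
; Camera clamping to an overlapped box is disconnected, leaving UpdateCamera empty.
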(event `UpdateAnimation`
  ;[1 1 1] Handle Animation
  (`PaperFlipbookComponent.SetFlipbook` (`self.Sprite`) (select `bool` (> (`KismetMathLibrary.VSize` (`self.GetVelocity`)) 0.0) :`false` "/Game/Game/Sprites/PlayerFlipbooks/A_Idle.A_Idle" :`true` "/Game/Game/Sprites/PlayerFlipbooks/A_Idle.A_Idle" :!type "PaperFlipbook Object Reference")))

(event `InputAction|Jump`
  (params (Key :type "Key Structure"))
  ;[1 1 1] Handle Jump
  (:`Pressed`
    (if (not (`|EnumEquality` (`self.State`) "NewEnumerator5")) :!label _label
      (`self.Jump`)
      (set `self.bCameraUpdated` false)))
  (:`Released`
    (`self.StopJumping` :!label _label_2)))

(event `InputTouch`
  (params (Location :type "Vector Structure") (FingerIndex :type "ETouchIndex Enum"))
  ;[1 1 1] Handle Jump
  (:`Pressed`
    (goto _label))
  (:`Released`
    (goto _label_2)))

(event `UpdateCamera`
  ;[1 1 1] Handle Camera Boundaries & Update Camera
)

(event `self.ReceiveBeginPlay`
  ;[1 1 1] Begin Play
  (bind _outactors (`GameplayStatics.GetAllActorsOfClass` "/Script/Engine.PlayerStart"))
  (for _array_element _outactors
    (if (== (`PlayerStart.PlayerStartTag` _array_element) "HUB")
      (`self.K2_TeleportTo` (`self.K2_GetActorLocation` _array_element))
      (`ActorComponent.SetIsReplicated` (`self.Sprite`) true))))

(event `Key|F`
  (params (Key :type "Key Structure"))
  (:`Pressed`
    (bind _outactors (`GameplayStatics.GetAllActorsOfClass` "/Script/Engine.PlayerStart"))
    (for _array_element _outactors
      (if (== (`PlayerStart.PlayerStartTag` _array_element) "Assassins")
        (`self.K2_TeleportTo` (`self.K2_GetActorLocation` _array_element))))))

(event `self.Box.OnComponentBeginOverlap`
  (params (OverlappedComponent :type "PrimitiveComponent Object Reference") (OtherActor :type "Actor Object Reference") (OtherComp :type "PrimitiveComponent Object Reference") (OtherBodyIndex :type Integer) (bFromSweep :type Boolean) (SweepResult :type "HitResult Structure (by ref)"))
  ;[1 1 1] Handle Camera Boundaries & Update Camera
  (bind _asbox_collision (cast `BoxComponent` OtherComp))
  (set `self.OutsideBox` _asbox_collision))

(event `Key|Z`
  (params (Key :type "Key Structure"))
  (:`Pressed`
    (`self.K2_TeleportTo` (-17899.0 0.0 4500.0))))

(event `InputAxis|MoveRight`
  (params (AxisValue :type "Float (single-precision)"))
  ;[1 1 1] Handle Movement
  (if (> AxisValue 0.0)
    (set `self.bisMovingRight` true)
    (elif (< AxisValue 0.0)
      (set `self.bisMovingRight` false)))
  (`self.AddMovementInput` (1.0 0.0 0.0) AxisValue)
  (set `self.bCameraUpdated` false))

(event `self.ReceiveTick`
  (params (DeltaSeconds :type "Float (single-precision)"))
  ;[1 1 1] Tick - Updates Animation and Camera
  (`self.UpdateAnimation`)
  (`/Engine/EditorBlueprintResources/StandardMacros.CompareFloat` (.x (`MovementComponent.Velocity` (`self.GetMovementComponent`)))
    (:`>`
      (`Controller.SetControlRotation` (`self.GetController`) (`KismetMathLibrary.MakeRotator` 0.0 0.0 180.0) :!label _label_3))
    (:`==`
      (if (`self.bisMovingRight`)
        (goto _label_3)
        (else
          (`Controller.SetControlRotation` (`self.GetController`) (`KismetMathLibrary.MakeRotator` 0.0) :!label _label_4))))
    (:`<`
      (goto _label_4))))

(event `Key|S`
  (params (Key :type "Key Structure"))
  ;[1 1 1] Spirit Slam
  (:`Pressed`
    (set `self.bDownHeld` true))
  (:`Released`
    (set `self.bDownHeld` false)))

(event `Key|E`
  (params (Key :type "Key Structure"))
  ;[1 1 1] Spirit Slam
  (:`Pressed`
    (if (`self.bDownHeld`)
      (if (`NavMovementComponent.IsFalling` (`self.CharacterMovement`))
        (`self.LaunchCharacter` (0.0 0.0 -2000.0) false true)))))

(event `Key|E`
  (params (Key :type "Key Structure"))
  (bind _capsulecomponent (`self.CapsuleComponent`))
  ;[1 1 1] Shadowstep
  (:`Pressed`
    (`PrimitiveComponent.SetCollisionObjectType` _capsulecomponent "ECC_GameTraceChannel1")
    (set `self.State` "NewEnumerator5")
    (`KismetSystemLibrary.Delay` 4.0)
    (`PrimitiveComponent.SetCollisionObjectType` _capsulecomponent "ECC_Pawn")
    (set `self.State` "NewEnumerator0")))

(fn `UserConstructionScript`)